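; Visualizer_BP is an actor that drops a new crate each time its SpawnNewElement event is called.
; DropNewCube spawns a CrateActor_BP above the visualizer at a random horizontal offset, at half the visualizer's scale, ignoring collisions.
; Each new crate is then attached to the visualizer, keeping its world transform.
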(event `self.SpawnNewElement`
  (`self.DropNewCube`))

(fn `DropNewCube`
  (bind _returnvalue (`|SpawnActorFromClass` "/Game/MeetupNov2019/Blueprints/CrateActor_BP.CrateActor_BP_C" (`KismetMathLibrary.MakeTransform` (+ (.location (`self.GetTransform`)) (`KismetMathLibrary.MakeVector` (`KismetMathLibrary.RandomFloatInRange` -50.0 50.0) (`KismetMathLibrary.RandomFloatInRange` -50.0 50.0) 150.0)) (struct) (* (.scale (`self.GetTransform`)) (0.5 0.5 0.5))) "AlwaysSpawn" "OverrideRootScale" null null))
  (`self.K2_AttachToActor` _returnvalue self "None" "KeepWorld" "KeepWorld" "KeepWorld" true))

(fn `UserConstructionScript`)